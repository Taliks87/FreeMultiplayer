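; BP_Player is the player character Blueprint for melee combat, with movement, attack, block, damage and death.
; Attacks play random montages, and LaunchAttack runs a server-side forward line trace that applies randomized damage unless the hit player blocks while roughly facing the attacker.
; Damage feeds the health component and plays random reactions, whose montages lock out movement and attacks, as does death.
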(event `InputAxis|MoveForward`
  (params (AxisValue :type "Float (single-precision)"))
  ;[1 1 1] Move
  (`self.CanMove`
    (:`Can`
      (`self.MoveForward` AxisValue))))

(event `InputAxis|MoveRight`
  (params (AxisValue :type "Float (single-precision)"))
  ;[1 1 1] Move
  (`self.CanMove`
    (:`Can`
      (`self.MoveRight` AxisValue))))

(event `InputAction|Attack`
  (params (Key :type "Key Structure"))
  ;[1 1 1] Attack
  (:`Pressed`
    (`self.Attack`)))

(event `Attack`
  ;[1 1 1] Attack
  (`self.CanAttack`
    (:`Can`
      (set `self.IsAttacking` true)
      (`self.AttackEffects`))))

(event `AttackEffects`
  (bind _speedattack (`self.SpeedAttack`))
  ;[1 1 1] Attack
  (bind _animation (`self.GetRandomAnimation` (`self.AnimAttacks`)))
  (bind _returnvalue (`self.PlayAnimMontage` _animation _speedattack))
  (`KismetSystemLibrary.Delay` (/ _returnvalue _speedattack))
  (set `self.IsAttacking` false))

(event `LaunchAttack`
  (bind _returnvalue (`self.K2_GetActorLocation`))
  ;[1 1 1] Attack
  (`/Engine/EditorBlueprintResources/ActorMacros.Switch Has Authority`
    (:`Authority`
      (bind _outhit (`KismetSystemLibrary.LineTraceSingleForObjects` _returnvalue (+ _returnvalue (* (`self.GetActorForwardVector`) (`self.AttackDistance`))) (`|MakeArray` "ObjectTypeQuery3" :!type "EObjectTypeQuery Enum")))
      (bind _isblocked (`self.AttackIsBlocked` (`.HitActor` (`GameplayStatics.BreakHitResult` _outhit))))
      (if (not _isblocked)
        (`GameplayStatics.ApplyDamage` (`.HitActor` (`GameplayStatics.BreakHitResult` _outhit)) (`self.GetDamage`))))))

(event `InputAction|Block`
  (params (Key :type "Key Structure"))
  ;[1 1 1] Block
  (:`Pressed`
    (`self.SetBlocking` true))
  (:`Released`
    (`self.SetBlocking` false)))

(event `SetBlocking`
  (params (isBlocking :type Boolean))
  ;[1 1 1] Block
  (set `self.IsBlocking` isBlocking))

(event `self.ReceiveAnyDamage`
  (params (Damage :type "Float (single-precision)") (DamageType :type "DamageType Object Reference") (InstigatedBy :type "Controller Object Reference") (DamageCauser :type "Actor Object Reference"))
  ;[1 1 1] Damage
  (`/Game/Characters/Blueprints/Components/BPC_Health.Damage` (`self.BPC_Health`) Damage)
  (`self.DamageEffects`))

(event `DamageEffects`
  ;[1 1 1] Damage
  (`KismetSystemLibrary.Delay` 0.1)
  (if (not (`self.IsDead`))
    (bind _animation (`self.GetRandomAnimation` (`self.AnimReacts`)))
    (`self.PlayAnimMontage` _animation)))

(event `self.BPC_Health.OnDead`
  ;[1 1 1] Death
  (`self.Death`))

(event `Death`
  ;[1 1 1] Death
  (set `self.IsDead` true))

(fn `AttackIsBlocked`
  (params (HitActor :type "Actor Object Reference"))
  (returns (IsBlocked :type Boolean))
  (bind _asbp_player (cast `/Game/Characters/Blueprints/Player/BP_Player` HitActor)
    (:`then`
      (return (and (`/Game/Characters/Blueprints/Player/BP_Player.IsBlocking` _asbp_player) (< (`KismetMathLibrary.Dot_VectorVector` (`self.GetActorForwardVector` HitActor) (`self.GetActorForwardVector`)) -0.75))))
    (:`CastFailed`
      (return false))))

(fn `GetDamage`
  (returns (Damage :type "Float (double-precision)"))
  (bind _basedamage (`self.BaseDamage`))
  (return (`KismetMathLibrary.RandomFloatInRange` (* _basedamage 0.5) (* _basedamage 1.5))))

(fn `GetRandomAnimation`
  (params (Animations :type "Array of AnimMontage Object Reference"))
  (returns (Animation :type "AnimMontage Object Reference"))
  (return (`|GetArrayItem` Animations (`KismetMathLibrary.RandomInteger` (`KismetArrayLibrary.Array_Length` Animations)))))

(fn `UserConstructionScript`)